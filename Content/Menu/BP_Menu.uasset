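; Card-based menu Blueprint that fades in from the camera fade, sets Game and UI input, and moves a camera between cards.
; Primary-finger touches become left-mouse presses on a WidgetInteraction component.
; ChangeCardFocus uses a timeline to lerp the camera to the target card's camera location.
; At the halfway point, DoOnce gates flip the new card and unflip the old one, with card 0 exempt from both.
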(event `self.ReceiveBeginPlay`
  (bind _returnvalue (`GameplayStatics.GetPlayerController` 0))
  (`PlayerCameraManager.StartCameraFade` :`self` (`GameplayStatics.GetPlayerCameraManager` 0) :`FromAlpha` 1.0 :`Duration` 1.0 :`bShouldFadeAudio` true :`bHoldWhenFinished` true)
  (`WidgetBlueprintLibrary.SetInputMode_GameAndUIEx` _returnvalue null)
  (bind _asjump_player_controller (cast `/Game/GameMode/JumpPlayerController` _returnvalue))
  (set `self.As Jump Player Controller` _asjump_player_controller))

(event `InputTouch`
  (params (Location :type "Vector Structure") (FingerIndex :type "ETouchIndex Enum"))
  (bind _returnvalue (== FingerIndex 0))
  (bind _widgetinteraction (`self.WidgetInteraction`))
  (:`Pressed`
    (if _returnvalue
      (`WidgetInteractionComponent.PressPointerKey` _widgetinteraction "LeftMouseButton")))
  (:`Released`
    (if _returnvalue
      (`WidgetInteractionComponent.ReleasePointerKey` _widgetinteraction "LeftMouseButton"))))

(event `ChangeCardFocus`
  (params (Card_ID :type Integer) (OldCard_ID :type Integer))
  (bind _cards (`self.Cards`))
  (bind _oldlocation (`self.OldLocation`))
  (bind _returnvalue (`SceneComponent.K2_GetComponentLocation` (`self.Camera`)))
  (bind _output (`|GetArrayItem` _cards Card_ID))
  (bind _returnvalue_2 (`SceneComponent.K2_GetComponentLocation` (`/Game/Menu/Card_BP.Camera` _output)))
  (set `self.OldLocation` _returnvalue)
  (bind (_direction _newtrack_0) (`Timeline|Lerp` :!via `PlayFromStart`)
    (:`Update`
      (`SceneComponent.K2_SetWorldLocation` (`self.Camera`) (`KismetMathLibrary.VLerp` _oldlocation _returnvalue_2 _newtrack_0) false false)
      (if (<= (`KismetMathLibrary.Vector_Distance` _returnvalue _returnvalue_2) (/ (`KismetMathLibrary.Vector_Distance` _oldlocation _returnvalue_2) 2.0))
        (if (not (== Card_ID 0))
          (`/Engine/EditorBlueprintResources/StandardMacros.DoOnce` false :!label _label
            (:`Completed`
              (`/Game/Menu/Card_BP.CardFlip` _output))))
        (`/Engine/EditorBlueprintResources/StandardMacros.DoOnce` false :!label _label_2
          (:`Completed`
            (if (not (== OldCard_ID 0))
              (`/Game/Menu/Card_BP.CardUnflip` (`|GetArrayItem` _cards OldCard_ID)))))
        (else
          (goto _label :!via `Reset`))))
    (:`Finished`
      (goto _label_2 :!via `Reset`))))

(fn `UserConstructionScript`)