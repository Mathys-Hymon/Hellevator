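; Menu confirmation card actor for a save slot, with a dynamic material on its plane and a Confirmation_UI widget.
; SaveNumber passes the slot number and itself to the widget, then a timeline lerps the card from its spawn transform to the target with slight random yaw.
; DeleteCard plays a second timeline back to the original transform, destroys the card on finish, and notifies the originating card via ConfirmationCardLeave.
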(event `self.ReceiveBeginPlay`
  (bind _returnvalue (`PrimitiveComponent.CreateDynamicMaterialInstance` (`self.Plane1`) 0 "/Game/Menu/Images/Cards/CardMat/Confirmation_MAT.Confirmation_MAT" "None"))
  (set `self.MAT_Card` _returnvalue))

(event `SaveNumber`
  (params (SaveNum :type Integer) (TargetTransform :type "Transform Structure") (CardREF :type "/Game/Menu/Card_BP Object Reference"))
  (set `self.Card REF` CardREF)
  (set `self.OriginalTransform` (`self.GetTransform`))
  (set `self.Target Transform` (`KismetMathLibrary.MakeTransform` (.location TargetTransform) (`KismetMathLibrary.MakeRotator` (.roll (.rotation TargetTransform)) (.pitch (.rotation TargetTransform)) (+ (.yaw (.rotation TargetTransform)) (`KismetMathLibrary.RandomFloatInRange` -10.0 10.0))) (.scale TargetTransform)))
  (bind _output_get (set `self.Save Num` SaveNum))
  (bind _asconfirmation_ui (cast `/Game/Menu/Widgets/Confirmation_UI` (`WidgetComponent.GetWidget` (`self.Widget1`))))
  (`/Game/Menu/Widgets/Confirmation_UI.GetSlotNumber` _asconfirmation_ui _output_get self)
  (`self.AnimCard`))

(event `AnimCard`
  (bind (_direction _newtrack_0) (`Timeline|Timeline`)
    (:`Update`
      (`SceneComponent.K2_SetWorldTransform` (`self.DefaultSceneRoot`) (`KismetMathLibrary.TLerp` (`self.OriginalTransform`) (`self.Target Transform`) _newtrack_0) false false))))

(event `DeleteCard`
  (`|ExecutionSequence`
    (:`then_0`
      (bind (_direction _newtrack_0) (`Timeline|Timeline_0` :!via `PlayFromStart`)
        (:`Update`
          (`SceneComponent.K2_SetWorldTransform` (`self.DefaultSceneRoot`) (`KismetMathLibrary.TLerp` (`self.Target Transform`) (`self.OriginalTransform`) _newtrack_0) false false))
        (:`Finished`
          (`self.K2_DestroyActor`))))
    (:`then_1`
      (`/Game/Menu/Card_BP.ConfirmationCard_Leave` (`self.Card REF`)))))

(fn `UserConstructionScript`)