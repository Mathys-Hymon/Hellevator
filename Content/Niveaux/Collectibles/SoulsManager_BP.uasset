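; SoulsManager_BP restores soul collectible state when a level starts, using the player's save data.
; After a one-second delay, it reads SpiritEnable from the PlayerCamera_Pawn's SaveGame for each Souls-tagged actor, indexed by soul Index plus LastMapMaxINDEX.
; Flagged souls are replaced by Souls_Catched_BP at a slightly offset transform.
; The others receive LastMapMaxINDEX through LastIndexAdding, the same offset used for the save lookup.
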(event `self.ReceiveBeginPlay`
  (`KismetSystemLibrary.Delay` 1.0)
  (bind _asplayer_camera_pawn (cast `/Game/Character/PlayerCamera_Pawn` (`GameplayStatics.GetPlayerPawn` 0)))
  (bind _output_get (set `self.player pawn ref` _asplayer_camera_pawn))
  (bind _outactors (`GameplayStatics.GetAllActorsWithTag` "Souls"))
  (for _array_element _outactors
    (bind _assouls_bp (cast `/Game/Niveaux/Collectibles/Souls_BP` _array_element))
    (if (`|GetArrayItem` (`/Game/GameMode/SaveMode/BP_SaveGame.SpiritEnable` (`/Game/Character/PlayerCamera_Pawn.SaveGame` _output_get)) (+ (`/Game/Niveaux/Collectibles/Souls_BP.Index` _assouls_bp) (`self.LastMapMaxINDEX`)))
      (bind (_returnvalue_location _returnvalue_rotation _returnvalue_scale) (`KismetMathLibrary.BreakTransform` (`SceneComponent.K2_GetComponentToWorld` (`/Game/Niveaux/Collectibles/Souls_BP.DefaultSceneRoot` _assouls_bp))))
      (`|SpawnActorFromClass` "/Game/Niveaux/Collectibles/Souls_Catched_BP.Souls_Catched_BP_C" (`KismetMathLibrary.MakeTransform` (- _returnvalue_location (-5.0 0.0 0.0)) _returnvalue_rotation _returnvalue_scale) "AlwaysSpawn" "OverrideRootScale" null null)
      (`self.K2_DestroyActor` _assouls_bp)
      (else
        (`/Game/Niveaux/Collectibles/Souls_BP.LastIndexAdding` _assouls_bp (`self.LastMapMaxINDEX`))))))

(fn `UserConstructionScript`)