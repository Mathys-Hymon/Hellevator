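; Soul collectible that the player picks up, reporting its index to PlayerCamera_Pawn through GetASpirit.
; On BeginPlay it derives that index from up to two digits in its own display name, and LastIndexAdding can offset it.
; A looping timeline bobs the flipbook vertically, with a random delay before each cycle to desynchronize instances.
; Overlap with Player_Pawn reports the index, plays the Falling flipbook once, then destroys the actor.
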(event `PlayTimeline`
  ;[1 1 1] BeginPlay
  (`KismetSystemLibrary.Delay` (`KismetMathLibrary.RandomFloatInRange` 0.0 0.3) :!label _label)
  (bind (_direction _newtrack_0) (`Timeline|Timeline` :!via `PlayFromStart`)
    (:`Update`
      (`SceneComponent.K2_SetRelativeLocation` (`self.PaperFlipbook`) (`KismetMathLibrary.MakeVector` 0.0 0.0 (`KismetMathLibrary.Lerp` 0.0 5.0 _newtrack_0)) false false))
    (:`Finished`
      (`self.PlayTimeline`))))

(event `self.ReceiveBeginPlay`
  (bind _indexconversion (`self.IndexConversion`))
  (bind _returnvalue (`KismetSystemLibrary.GetDisplayName` self))
  (bind _returnvalue_2 (`KismetStringLibrary.Conv_StringToInt` (`KismetTextLibrary.Conv_TextToString` (`|FormatText` "{number1}{number2}" (`|GetArrayItem` _indexconversion) (`|GetArrayItem` _indexconversion 1)))))
  ;[1 1 1] BeginPlay
  (for _index (range (+ (`KismetStringLibrary.Len` _returnvalue) 1))
    (bind _returnvalue_3 (`KismetStringLibrary.GetCharacterAsNumber` _returnvalue _index))
    (if (and (<= _returnvalue_3 57) (>= _returnvalue_3 48))
      (bind _indexoutput (`self.IndexConvertor` _returnvalue_3))
      (`KismetArrayLibrary.Array_Add` (`self.IndexConversion`) _indexoutput)))
  (set `self.Index` (`KismetMathLibrary.SelectInt` (/ _returnvalue_2 10) _returnvalue_2 (== (`KismetArrayLibrary.Array_Length` _indexconversion) 1)))
  (goto _label))

(event `LastIndexAdding`
  (params (NewParam :type Integer))
  (set `self.Index` (+ (`self.Index`) NewParam)))

(event `self.ReceiveActorBeginOverlap`
  (params (OtherActor :type "Actor Object Reference"))
  (bind _paperflipbook (`self.PaperFlipbook`))
  (if (== (`GameplayStatics.GetObjectClass` OtherActor) "/Game/Character/Player_Pawn.Player_Pawn_C")
    (bind _asplayer_camera_pawn (cast `/Game/Character/PlayerCamera_Pawn` (`GameplayStatics.GetPlayerPawn` 0)))
    (`/Game/Character/PlayerCamera_Pawn.GetASpirit` _asplayer_camera_pawn (`self.Index`))
    (`PaperFlipbookComponent.SetFlipbook` _paperflipbook "/Game/Character/Sprites/Jump/Falling.Falling")
    (`PaperFlipbookComponent.SetLooping` _paperflipbook false)
    (`KismetSystemLibrary.Delay` (`PaperFlipbookComponent.GetFlipbookLength` _paperflipbook))
    (`self.K2_DestroyActor`)))

(fn `IndexConvertor`
  (params (IndexInput :type Integer))
  (returns (IndexOutput :type Integer))
  (if (== IndexInput 48)
    (return 0)
    (elif (== IndexInput 49)
      (return 1)
      (elif (== IndexInput 50)
        (return 2)
        (elif (== IndexInput 51)
          (return 3)
          (elif (== IndexInput 52)
            (return 4)
            (elif (== IndexInput 53)
              (return 5)
              (elif (== IndexInput 54)
                (return 6)
                (elif (== IndexInput 55)
                  (return 7)
                  (elif (== IndexInput 56)
                    (return 8)
                    (elif (== IndexInput 57)
                      (return 9))))))))))))

(fn `UserConstructionScript`)