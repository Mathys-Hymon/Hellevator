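; Shopkeeper actor that starts a dialogue when the player pawn enters its trigger box.
; On overlap it scans the box for a Player_Pawn and, through a DoOnce, passes its English and French dialogue, portrait and itself to JumpPlayerController's DialogueCE, flagged as repeatable.
; The construction script sizes the trigger and flips the character's yaw to face either side.
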(event `self.ReceiveBeginPlay`
  (bind _asjump_player_controller (cast `/Game/GameMode/JumpPlayerController` (`GameplayStatics.GetPlayerController` 0)))
  (set `self.As Jump Player Controller` _asjump_player_controller))

(event `self.BoxTriggerZone.OnComponentBeginOverlap`
  (params (OverlappedComponent :type "PrimitiveComponent Object Reference") (OtherActor :type "Actor Object Reference") (OtherComp :type "PrimitiveComponent Object Reference") (OtherBodyIndex :type Integer) (bFromSweep :type Boolean) (SweepResult :type "HitResult Structure (by ref)"))
  (for _array_element (`PrimitiveComponent.GetOverlappingActors` (`self.BoxTriggerZone`) null)
    (if (== (`GameplayStatics.GetObjectClass` _array_element) "/Game/Character/Player_Pawn.Player_Pawn_C")
      (`|ExecutionSequence`
        (:`then_0`
          (break))
        (:`then_1`
          (`/Engine/EditorBlueprintResources/StandardMacros.DoOnce` false
            (:`Completed`
              (`/Game/Dialogue_System/BP/Dialogue_BPI.DialogueCE` (`self.As Jump Player Controller`) (`self.DialogueEN`) (`self.DialogueFR`) (`self.Chracter Picture`) "ShopKeeper" true self))))))))

(event `/Game/Dialogue_System/BP/Dialogue_BPI.FinishPlaying`)

(fn `UserConstructionScript`
  (`BoxComponent.SetBoxExtent` (`self.BoxTriggerZone`) (`self.TriggerSize`) true)
  (`SceneComponent.K2_SetWorldRotation` (`self.Character`) (`KismetMathLibrary.MakeRotator` 0.0 0.0 (`KismetMathLibrary.SelectFloat` 90.0 -90.0 (`self.ChangeLookSide`))) false false))